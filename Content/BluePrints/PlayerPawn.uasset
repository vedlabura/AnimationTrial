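; Player character with touch-drag camera look, jumping and a pickup prompt for rifles.
; Overlapping a BP_Rifle creates a PickUpButton widget, displayed only when locally controlled; any end overlap removes the first such widget found.
; Tick polls the Movefinger touch from MyPlayerController and turns scaled frame-to-frame movement into yaw and pitch, using WasTouched to reset the origin on each new press.
; Space bar triggers Jump.
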(event `Key|SpaceBar`
  (params (Key :type "Key Structure"))
  (:`Pressed`
    (`self.Jump`)))

(event `self.CapsuleComponent.OnComponentBeginOverlap`
  (params (OverlappedComponent :type "PrimitiveComponent Object Reference") (OtherActor :type "Actor Object Reference") (OtherComp :type "PrimitiveComponent Object Reference") (OtherBodyIndex :type Integer) (bFromSweep :type Boolean) (SweepResult :type "HitResult Structure (by ref)"))
  (cast `/Game/BluePrints/BP_Rifle` OtherActor)
  (bind _returnvalue (`|CreateWidget` "/Game/BluePrints/PickUpButton.PickUpButton_C" (`GameplayStatics.GetPlayerController` 0)))
  (if (`self.IsLocallyControlled`)
    (`UserWidget.AddToViewport` _returnvalue 0)))

(event `self.CapsuleComponent.OnComponentEndOverlap`
  (params (OverlappedComponent :type "PrimitiveComponent Object Reference") (OtherActor :type "Actor Object Reference") (OtherComp :type "PrimitiveComponent Object Reference") (OtherBodyIndex :type Integer))
  (bind _foundwidgets (`WidgetBlueprintLibrary.GetAllWidgetsOfClass` "/Game/BluePrints/PickUpButton.PickUpButton_C"))
  (if (`self.IsLocallyControlled`)
    (`Widget.RemoveFromParent` (`|GetArrayItem` _foundwidgets))))

(event `self.ReceiveTick`
  (params (DeltaSeconds :type "Float (single-precision)"))
  (bind _returnvalue (`GameplayStatics.GetPlayerController` 0))
  (bind _asmy_player_controller (cast `/Game/BluePrints/MyPlayerController` _returnvalue))
  (bind (_locationx _locationy _biscurrentlypressed) (`PlayerController.GetInputTouchState` _returnvalue (`/Game/BluePrints/MyPlayerController.movefinger` _asmy_player_controller)))
  (if _biscurrentlypressed
    (if (`self.Was Touched`)
      (`self.AddControllerYawInput` (/ (- _locationx (`self.X`)) 5.0))
      (`self.AddControllerPitchInput` (/ (- _locationy (`self.Y`)) 5.0))
      (set `self.Y` _locationy)
      (set `self.X` _locationx)
      (else
        (set `self.Was Touched` true)
        (set `self.Y` _locationy)
        (set `self.X` _locationx)))
    (else
      (set `self.Was Touched` false))))

(fn `UserConstructionScript`)