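; MyPawnbp is a pawn Blueprint that shows a pickup button when it touches a rifle.
; A capsule overlap with a BP_Rifle creates a new PickUpButton widget owned by player controller 0, then adds it to the viewport only if the pawn is locally controlled.
; Tick prints the controller's control rotation on screen every frame as debug output.
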(event `self.ReceiveTick`
  (params (DeltaSeconds :type "Float (single-precision)"))
  (`KismetSystemLibrary.PrintString` (`KismetStringLibrary.Conv_RotatorToString` (`Controller.GetControlRotation` (`self.GetController`))) true true (struct :`G` 0.66 :`B` 1.0 :`A` 1.0) 0.0))

(event `self.CapsuleComponent.OnComponentBeginOverlap`
  (params (OverlappedComponent :type "PrimitiveComponent Object Reference") (OtherActor :type "Actor Object Reference") (OtherComp :type "PrimitiveComponent Object Reference") (OtherBodyIndex :type Integer) (bFromSweep :type Boolean) (SweepResult :type "HitResult Structure (by ref)"))
  (cast `/Game/BluePrints/BP_Rifle` OtherActor)
  (bind _returnvalue (`|CreateWidget` "/Game/BluePrints/PickUpButton.PickUpButton_C" (`GameplayStatics.GetPlayerController` 0)))
  (if (`self.IsLocallyControlled`)
    (`UserWidget.AddToViewport` _returnvalue 0)))

(fn `UserConstructionScript`)