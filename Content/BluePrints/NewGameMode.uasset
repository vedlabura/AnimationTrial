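; Game mode for a two-team match that assigns players to alternating teams on login, using a player count kept in NewGameStateBase.
; At start it spawns two BP_Rifle actors at fixed locations.
; Died calls Won on the game state if red or blue score equals two, otherwise it respawns the pawn at one fixed point and re-possesses it.
; AnyDamage only prints the damage; a team-flipping branch is left unconnected.
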(event `self.K2_PostLogin`
  (params (NewPlayer :type "PlayerController Object Reference"))
  (bind _asnew_game_state_base (cast `/Game/BluePrints/NewGameStateBase` (`GameplayStatics.GetGameState`)))
  (bind _result (`/Engine/EditorBlueprintResources/StandardMacros.IncrementInt` (`/Game/BluePrints/NewGameStateBase.NoOfPLayers` _asnew_game_state_base))
    (:`  `
      (bind _asmy_player_controller (cast `/Game/BluePrints/MyPlayerController` NewPlayer))
      (set `/Game/BluePrints/MyPlayerController.TEAM` (== (mod _result 2) 1) _asmy_player_controller))))

(event `self.ReceiveBeginPlay`
  (`|SpawnActorFromClass` "/Game/BluePrints/BP_Rifle.BP_Rifle_C" (`KismetMathLibrary.MakeTransform` (-2992.0 2107.0 -8.0)) "AlwaysSpawn" "OverrideRootScale" null null)
  (`|SpawnActorFromClass` "/Game/BluePrints/BP_Rifle.BP_Rifle_C" (`KismetMathLibrary.MakeTransform` (8172.0 350.0 18.0)) "AlwaysSpawn" "OverrideRootScale" null null))

(event `self.ReceiveAnyDamage`
  (params (Damage :type "Float (single-precision)") (DamageType :type "DamageType Object Reference") (InstigatedBy :type "Controller Object Reference") (DamageCauser :type "Actor Object Reference"))
  (`KismetSystemLibrary.PrintString` (`KismetStringLibrary.Conv_DoubleToString` Damage) true true (struct :`G` 0.66 :`B` 1.0 :`A` 1.0) 19.0))

(event `Died`
  (params (PlayerPawn :type "/Game/BluePrints/PlayerPawn Object Reference"))
  (bind _returnvalue (`Pawn.GetController` PlayerPawn))
  (bind _asnew_game_state_base (cast `/Game/BluePrints/NewGameStateBase` (`GameplayStatics.GetGameState`)))
  (if (== (`/Game/BluePrints/NewGameStateBase.RedScore` _asnew_game_state_base) 2)
    (bind _asnew_game_state_base_2 (cast `/Game/BluePrints/NewGameStateBase` (`GameplayStatics.GetGameState`) :!label _label))
    (`/Game/BluePrints/NewGameStateBase.Won` _asnew_game_state_base_2)
    (elif (== (`/Game/BluePrints/NewGameStateBase.BlueScore` _asnew_game_state_base) 2)
      (goto _label)
      (else
        (bind _output_get (set `self.Dying controller` _returnvalue))
        (`self.K2_DestroyActor` PlayerPawn)
        (bind _returnvalue_2 (`|SpawnActorFromClass` "/Game/BluePrints/PlayerPawn.PlayerPawn_C" (`KismetMathLibrary.MakeTransform` (8000.0 350.0 18.0)) "AlwaysSpawn" "OverrideRootScale" null null))
        (`Controller.Possess` _returnvalue _returnvalue_2)
        (`Controller.Possess` _output_get _returnvalue_2)))))

(fn `UserConstructionScript`)