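; Main menu actor that rotates around its yaw axis as a finger drags horizontally across the screen.
; Each Tick it polls the player controller's first touch and records the X position when a press begins.
; While the press holds, it applies the scaled frame-to-frame X change as local yaw rotation, turning opposite in sign to the drag, and resets the touch flag on release.
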(event `self.ReceiveTick`
  (params (DeltaSeconds :type "Float (single-precision)"))
  (bind (_locationx _locationy _biscurrentlypressed) (`PlayerController.GetInputTouchState` (`GameplayStatics.GetPlayerController` 0) "Touch1"))
  (if _biscurrentlypressed
    (if (`self.wasTouched`)
      (`self.K2_AddActorLocalRotation` (`KismetMathLibrary.MakeRotator` 0.0 0.0 (/ (- (`self.X`) _locationx) 5.0)))
      (set `self.X` _locationx)
      (else
        (set `self.wasTouched` true)
        (set `self.X` _locationx)))
    (else
      (set `self.wasTouched` false))))

(fn `UserConstructionScript`)