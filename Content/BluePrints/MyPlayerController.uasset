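; Player controller Blueprint that sets up the on-screen UI and tracks which touch finger is used for aiming.
; On BeginPlay it creates a BP_UiLayout and a HealthWidget for player 0, adds both to the viewport and stores references to them.
; A touch press on the right half of the viewport records that finger index as AimFinger.
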(event `self.ReceiveBeginPlay`
  (bind _returnvalue (`GameplayStatics.GetPlayerController` 0))
  (`/Engine/EditorBlueprintResources/ActorMacros.Switch Has Authority`
    (:`Authority`
      _)
    (:`Remote`
      _))
  (bind _returnvalue_2 (`|CreateWidget` "/Game/BluePrints/BP_UiLayout.BP_UiLayout_C" _returnvalue))
  (`UserWidget.AddToViewport` _returnvalue_2 0)
  (set `self.WidgetVar` _returnvalue_2)
  (bind _returnvalue_3 (`|CreateWidget` "/Game/UI/HealthWidget.HealthWidget_C" _returnvalue))
  (`UserWidget.AddToViewport` _returnvalue_3 0)
  (set `self.WidgetMove` _returnvalue_3))

(event `InputTouch`
  (params (Location :type "Vector Structure") (FingerIndex :type "ETouchIndex Enum"))
  (:`Pressed`
    (if (> Location_X (`KismetMathLibrary.Conv_IntToDouble` (/ (`self.GetViewportSize`) 2)))
      (set `self.AimFinger` FingerIndex))))

(fn `UserConstructionScript`)